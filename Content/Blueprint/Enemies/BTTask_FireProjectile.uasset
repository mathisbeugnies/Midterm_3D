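; Behavior tree task that makes an enemy character fire a projectile at the player's location.
; It turns the pawn toward the blackboard location, then spawns BP_Projectile at the muzzle point and decrements the enemy's ammo.
; It fails when ammo is already empty; spending the last round clears the can-see-player key and finishes with success.
; A shot that leaves ammo remaining never calls FinishExecute.
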(event `self.ReceiveExecuteAI`
  (params (OwnerController :type "AIController Object Reference") (ControlledPawn :type "Pawn Object Reference"))
  (`Actor.K2_SetActorRotation` ControlledPawn (`KismetMathLibrary.FindLookAtRotation` (`Actor.K2_GetActorLocation` ControlledPawn) (`BTFunctionLibrary.GetBlackboardValueAsVector` (`self.PlayerLocationKey`))) false)
  (bind _asbp_enemy_character (cast `/Game/Blueprint/Enemies/BP_EnemyCharacter` ControlledPawn))
  (bind _enemyammo (`/Game/Blueprint/Enemies/BP_EnemyCharacter.EnemyAmmo` _asbp_enemy_character))
  (if (== _enemyammo 0)
    (`self.FinishExecute` false)
    (else
      (`|SpawnActorFromClass` "/Game/Blueprint/BP_Projectile.BP_Projectile_C" (`SceneComponent.K2_GetComponentToWorld` (`/Game/Blueprint/Enemies/BP_EnemyCharacter.MuzzlePoint` _asbp_enemy_character)) "Undefined" "MultiplyWithRoot" null null)
      (bind _output_get (set `/Game/Blueprint/Enemies/BP_EnemyCharacter.EnemyAmmo` (- _enemyammo 1) _asbp_enemy_character))
      (if (== _output_get 0)
        (`BTFunctionLibrary.SetBlackboardValueAsBool` (`self.CanSeePlayerKey`))
        (`self.FinishExecute` true)))))