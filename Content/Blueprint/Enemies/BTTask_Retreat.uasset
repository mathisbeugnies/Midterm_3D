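; Behavior Tree task that makes an enemy pawn retreat directly away from the player.
; It reads the player location from the blackboard and offsets the pawn's position a fixed distance along the opposite direction.
; The resulting point is written to the target move location key and also computed for AI MoveTo, without a navmesh query.
; The task finishes as success or failure according to the move result.
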(event `self.ReceiveExecuteAI`
  (params (OwnerController :type "AIController Object Reference") (ControlledPawn :type "Pawn Object Reference"))
  (bind _returnvalue (`Actor.K2_GetActorLocation` ControlledPawn))
  (bind _returnvalue_2 (`AIBlueprintHelperLibrary.GetBlackboard` OwnerController))
  (bind _returnvalue_3 (+ _returnvalue (* (`KismetMathLibrary.Normal` (- _returnvalue (`BlackboardComponent.GetValueAsVector` _returnvalue_2 (`.SelectedKeyName` (break `BlackboardKeySelector` (`self.PlayerLocationKey`)))))) 1200.0)))
  (`BlackboardComponent.SetValueAsVector` _returnvalue_2 (`.SelectedKeyName` (break `BlackboardKeySelector` (`self.TargetMoveLocationKey`))) _returnvalue_3)
  (`|AIMoveTo` ControlledPawn _returnvalue_3 null 20.0
    (:`OnSuccess`
      (`self.FinishExecute` true))
    (:`OnFail`
      (`self.FinishExecute` false))))